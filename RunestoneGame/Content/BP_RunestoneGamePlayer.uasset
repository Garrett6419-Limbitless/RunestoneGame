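; BP_RunestoneGamePlayer is a numbered player in the runestone game who paints on RuneCanvas actors with a cursor.
; Tick sets a viewport-scaled cursor position from the mouse or PlayerRotation aim and moves the WBP_PaintCursor widget, finding it if unset.
; Paint and MediumFlex inputs trace along the camera forward from raw cursor coordinates, then draw the brush texture at the hit's collision UV.
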(event `EnhancedInput|/Game/IA_Paint`
  (params (ActionValue :type Boolean) (ElapsedSeconds :type "Float (double-precision)") (TriggeredSeconds :type "Float (double-precision)") (InputAction :type "InputAction Object Reference" :default "/Game/IA_Paint.IA_Paint"))
  (bind (_currentcursorposition_x _currentcursorposition_y) (`KismetMathLibrary.BreakVector2D` (`self.CurrentCursorPosition`)))
  (:`Triggered`
    (if ActionValue
      (bind _outhit (`KismetSystemLibrary.LineTraceSingle` (`KismetMathLibrary.MakeVector` _currentcursorposition_x _currentcursorposition_y) (+ (`KismetMathLibrary.MakeVector` _currentcursorposition_x _currentcursorposition_y) (* (`self.GetActorForwardVector` (`GameplayStatics.GetPlayerCameraManager` (`self.PlayerNumber`))) 1500.0)) "TraceTypeQuery1" :!label _label))
      (bind _asrune_canvas (cast `/Game/Blueprints/RuneCanvas` (`.HitActor` (`GameplayStatics.BreakHitResult` _outhit))))
      (`/Game/Blueprints/RuneCanvas.DrawBrush` _asrune_canvas (`self.PaintBrushTexture`) (`self.PaintBrushSize`) (`GameplayStatics.FindCollisionUV` _outhit)))))

(event `EnhancedInput|/LimbitlessBluetoothPlugin/InputActions/IA_MediumFlex`
  (params (ActionValue :type Boolean) (ElapsedSeconds :type "Float (double-precision)") (TriggeredSeconds :type "Float (double-precision)") (InputAction :type "InputAction Object Reference" :default "/LimbitlessBluetoothPlugin/InputActions/IA_MediumFlex.IA_MediumFlex"))
  (:`Triggered`
    (if ActionValue
      (goto _label))))

(event `self.ReceiveBeginPlay`)

(event `self.ReceiveTick`
  (params (DeltaSeconds :type "Float (single-precision)"))
  (bind (_locationx _locationy) (`PlayerController.GetMousePosition` (`GameplayStatics.GetPlayerController` (`self.PlayerNumber`))))
  ;[1 1 1] Set The Cursor position with either the mouse or the player rotation component
  (`/Engine/EditorBlueprintResources/StandardMacros.IsValid` (`self.Cursor`)
    (:`Is Valid`
      (if (`self.bUseMouseInput`)
        (bind _output_get (set `self.CurrentCursorPosition` (/ (* (`KismetMathLibrary.MakeVector2D` _locationx _locationy) (4.0 1.0)) (`WidgetLayoutLibrary.GetViewportSize`))))
        (else
          (set `self.CurrentCursorPosition` (/ (`PlayerRotationComponent.GetAimPosition` (`self.PlayerRotation`)) (`WidgetLayoutLibrary.GetViewportSize`)))))
      (`/Game/Blueprints/WBP_PaintCursor.MoveCursor` (`self.Cursor`) (`self.PlayerNumber`) _output_get))
    (:`Is Not Valid`
      (bind _foundwidgets (`WidgetBlueprintLibrary.GetAllWidgetsOfClass` "/Game/Blueprints/WBP_PaintCursor.WBP_PaintCursor_C" false))
      (set `self.Cursor` (`|GetArrayItem` _foundwidgets)))))

(event `SetCursor`
  (params (Cursor :type "/Game/Blueprints/WBP_PaintCursor Object Reference"))
  (bind (_returnvalue_x _returnvalue_y) (`KismetMathLibrary.BreakVector2D` (* (`WidgetLayoutLibrary.GetViewportSize`) (0.5 0.5))))
  (`PlayerController.SetMouseLocation` (`GameplayStatics.GetPlayerController` (`self.PlayerNumber`)) (`KismetMathLibrary.FTrunc` _returnvalue_x) (`KismetMathLibrary.FTrunc` _returnvalue_y))
  (set `self.Cursor` Cursor))

(fn `UserConstructionScript`)